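; Dummy enemy AI that patrols random reachable points, detects and chases pawns, and deals contact damage to the player.
; Pawn sensing messages the seen pawn to start detection, using a retriggerable delay to stop it once sightings lapse; StartChase/StopChase toggle pursuit.
; Overlapping HitRange loops cooldown-gated attacks on the player.
; Damage feeds BPCEnemyStats, whose death event triggers ragdoll; a camera-facing health bar and debug self-damage key are included.
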(event `self.ReceiveBeginPlay`
  (bind _aswbp_enemy_health_bar (cast `/Game/UI/WBP_EnemyHealthBar` (`WidgetComponent.GetWidget` (`self.HealthBarWidget`))))
  (set `self.DummyHealthBarWidget` _aswbp_enemy_health_bar)
  (add `/Game/PlayerBlueprints/BPC_EnemyStats.OnDeath` (`self.BPC_EnemyStats`) (delegate `OnDeath_Event`))
  (`self.Patrol`))

(event `OnDeath_Event`
  (`self.Death`))

(event `Key|Subtract`
  (params (Key :type "Key Structure"))
  (:`Pressed`
    (`GameplayStatics.ApplyDamage` self 25.0)))

(event `self.ReceiveAnyDamage`
  (params (Damage :type "Float (single-precision)") (DamageType :type "DamageType Object Reference") (InstigatedBy :type "Controller Object Reference") (DamageCauser :type "Actor Object Reference"))
  ; Damage System
  (if (`self.Alive?`)
    (`/Game/PlayerBlueprints/BPC_EnemyStats.UpdateTotalHealth` (`self.BPC_EnemyStats`) Damage)))

(event `self.ReceiveTick`
  (params (DeltaSeconds :type "Float (single-precision)"))
  (`SceneComponent.K2_SetWorldRotation` (`self.HealthBarWidget`) (`KismetMathLibrary.FindLookAtRotation` (`SceneComponent.K2_GetComponentLocation` (`self.HealthBarWidget`)) (`SceneComponent.K2_GetComponentLocation` (`PlayerCameraManager.TransformComponent` (`GameplayStatics.GetPlayerCameraManager` 0)))) false false))

(event `Death`
  (bind _mesh (`self.Mesh`))
  ; Death Event
  (set `self.Alive?` false)
  (`PrimitiveComponent.SetSimulatePhysics` (`self.Mesh`) true)
  (`SkeletalMeshComponent.SetPhysicsBlendWeight` _mesh 1.0)
  (`PrimitiveComponent.SetCollisionEnabled` _mesh "QueryAndPhysics")
  (`PrimitiveComponent.SetCollisionEnabled` (`self.CapsuleComponent`) "NoCollision")
  (`/Game/UI/BP_DetectionInterface.StopDetection`)
  (`ActorComponent.K2_DestroyComponent` (`self.Hit Range`)))

(event `self.Hit Range.OnComponentBeginOverlap`
  (params (OverlappedComponent :type "PrimitiveComponent Object Reference") (OtherActor :type "Actor Object Reference") (OtherComp :type "PrimitiveComponent Object Reference") (OtherBodyIndex :type Integer) (bFromSweep :type Boolean) (SweepResult :type "HitResult Structure (by ref)"))
  ; NPC Damage
  (bind _asbp_first_person_character (cast `/Game/FirstPerson/Blueprints/BP_FirstPersonCharacter` OtherActor))
  (bind _output_get (set `self.As BP First Person Character` _asbp_first_person_character))
  (if (not (`/Game/FirstPerson/Blueprints/BP_FirstPersonCharacter.IsDead?` _output_get))
    (set `self.HitRange?` true)
    (if (and (`self.HitRange?`) (!= (`self.AttackCooldown?`) true)) :!label _label
      (`GameplayStatics.ApplyDamage` _output_get 25.0)
      (set `self.AttackCooldown?` true)
      (`KismetSystemLibrary.RetriggerableDelay` 1.5)
      (set `self.AttackCooldown?` false)
      (goto _label))))

(event `self.Hit Range.OnComponentEndOverlap`
  (params (OverlappedComponent :type "PrimitiveComponent Object Reference") (OtherActor :type "Actor Object Reference") (OtherComp :type "PrimitiveComponent Object Reference") (OtherBodyIndex :type Integer))
  ; NPC Damage
  (cast `/Game/FirstPerson/Blueprints/BP_FirstPersonCharacter` OtherActor)
  (set `self.HitRange?` false))

(event `Patrol`
  ; Detection and Patrol
  (if (`self.Alive?`) :!label _label_2
    (if (not (`self.ShouldChase?`))
      (`|AIMoveTo` self (`NavigationSystemV1.K2_GetRandomReachablePointInRadius` (`self.K2_GetActorLocation`) (`self.Radius`) null null) null (`self.Stop Distance`)
        (:`then`
          (`KismetSystemLibrary.Delay` (`KismetMathLibrary.RandomFloatInRange` 4.0 8.0))
          (goto _label_2))))))

(event `self.PawnSensing.OnSeePawn`
  (params (Pawn :type "Pawn Object Reference"))
  ; Detection and Patrol
  (if (`self.Alive?`)
    (`|ExecutionSequence`
      (:`then_0`
        (`|ExecutionSequence`
          (:`then_0`
            (`/Engine/EditorBlueprintResources/StandardMacros.DoOnce` false :!label _label_3
              (:`Completed`
                (message `/Game/UI/BP_DetectionInterface.StartDetection` Pawn self))))
          (:`then_1`
            (if (`self.ShouldChase?`)
              (`|AIMoveTo` self (0.0 0.0 0.0) Pawn)))))
      (:`then_1`
        (`KismetSystemLibrary.RetriggerableDelay` 0.5)
        (message `/Game/UI/BP_DetectionInterface.StopDetection` Pawn)
        (goto _label_3 :!via `Reset`)))))

(event `self.StartChase`
  ; Detection and Patrol
  (set `self.ShouldChase?` true))

(event `self.StopChase`
  ; Detection and Patrol
  (set `self.ShouldChase?` false)
  (`|AIMoveTo` self (0.0 0.0 0.0) self))

(fn `UserConstructionScript`)