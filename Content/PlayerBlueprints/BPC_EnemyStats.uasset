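; BPC_EnemyStats is an actor component that tracks health and death for the dummy AI enemy.
; On BeginPlay it casts its owner to BP_DummyAi and fills that actor's health bar widget from the health ratio.
; UpdateTotalHealth subtracts damage, clamps to a hardcoded maximum rather than MaxHealth, prints the value, refreshes the bar and calls the OnDeath dispatcher at zero health.
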(event `self.ReceiveBeginPlay`
  (bind _asbp_dummy_ai (cast `/Game/Ai/BP_DummyAi` (`self.GetOwner`)))
  (bind _output_get (set `self.As BP Dummy Ai` _asbp_dummy_ai))
  (`ProgressBar.SetPercent` (`/Game/UI/WBP_EnemyHealthBar.HealthBar` (`/Game/Ai/BP_DummyAi.DummyHealthBarWidget` _output_get)) (/ (`self.CurrentHealth`) (`self.MaxHealth`))))

(fn `UpdateTotalHealth`
  (params (Damage :type "Float (double-precision)"))
  (bind _output_get (set `self.CurrentHealth` (`KismetMathLibrary.FClamp` (- (`self.CurrentHealth`) Damage) 0.0 75.0)))
  (`KismetSystemLibrary.PrintString` (`KismetStringLibrary.Conv_DoubleToString` _output_get))
  (`ProgressBar.SetPercent` (`/Game/UI/WBP_EnemyHealthBar.HealthBar` (`/Game/Ai/BP_DummyAi.DummyHealthBarWidget` (`self.As BP Dummy Ai`))) (/ _output_get (`self.MaxHealth`)))
  (if (<= _output_get 0.0)
    (`self.OnDeath`)))